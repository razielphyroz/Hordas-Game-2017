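; EnemyDeath is an enemy actor that periodically fires DeathProjectile toward the player character referenced by Personagem.
; While ReadyToPlay is set, a Delay on Tick paces a random roll to about once per second, with a one-in-five chance to shoot.
; Projectiles spawn at the enemy's XY and a fixed world height, using a look-at rotation with pitch zeroed to keep the aim horizontal.
; Hit events are forwarded to OnHit.
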(event EventBeginPlay)

(event Collision|EventActorBeginOverlap
  (params (OtherActor :type Actor%20Object%20Reference)))

(event EventTick
  (params (DeltaSeconds :type Float%20%28single-precision%29))
  (bind _returnvalue (Transformation|GetActorLocation))
  (bind _personagem (Variables|Default|GetPersonagem))
  (bind _returnvalue_2 (Transformation|GetActorLocation _personagem))
  (bind (_x _y) (Math|Vector|BreakVector _returnvalue))
  (bind _returnvalue_3 (Math|Rotator|FindLookatRotation _returnvalue _returnvalue_2))
  (bind (_roll _pitch _yaw) (Math|Rotator|BreakRotator _returnvalue_3))
  (if (Variables|Default|GetReadyToPlay)
    (Utilities|FlowControl|Delay 1.0)
    (switch int (Math|Random|RandomInteger 5)
      (:0
        (Game|SpawnActorfromClass "/Game/Blueprints/Projectiles/EnemyProjectiles/DeathProjectile.DeathProjectile_C" (Math|Transform|MakeTransform (Math|Vector|MakeVector _x _y 225.0) (Math|Rotator|MakeRotator _roll 0.0 _yaw) "0.500000,1,0.500000") "AdjustIfPossibleButAlwaysSpawn" 0 0)))))

(event Collision|EventHit
  (params (MyComp :type Primitive%20Component%20Object%20Reference) (Other :type Actor%20Object%20Reference) (OtherComp :type Primitive%20Component%20Object%20Reference) (bSelfMoved :type Boolean) (HitLocation :type Vector :default "0, 0, 0") (HitNormal :type Vector :default "0, 0, 0") (NormalImpulse :type Vector :default "0, 0, 0") (Hit :type Hit%20Result%20Structure%20%28by%20ref%29))
  (Class|Enemy|OnHit Other))

(fn ConstructionScript)