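; UserBP is a player-input Blueprint that fires Projectile actors toward the mouse cursor while the left mouse button is held.
; The button opens and closes a Gate on Tick, with a short Delay throttling the fire rate.
; Each shot spawns at the controlled pawn's XY and aims at the cursor's visibility-trace hit, both flattened to a fixed height so shots travel horizontally.
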(event EventBeginPlay)

(event Collision|EventActorBeginOverlap
  (params (OtherActor :type Actor%20Object%20Reference)))

(event EventTick
  (params (DeltaSeconds :type Float%20%28single-precision%29))
  (bind _returnvalue (Game|GetPlayerController 0))
  (bind _returnvalue_2 (Pawn|GetControlledPawn _returnvalue))
  (bind _hitresult (Game|Player|GetHitResultUnderCursorbyChannel _returnvalue "TraceTypeQuery1" true))
  (bind _returnvalue_3 (Transformation|GetActorLocation _returnvalue_2))
  (bind _location (Collision|BreakHitResult _hitresult))
  (bind (_x _y) (Math|Vector|BreakVector _location))
  (bind (_x_2 _y_2) (Math|Vector|BreakVector _returnvalue_3))
  (Utilities|FlowControl|Gate true
    (:Exit
      (Utilities|FlowControl|Delay 0.2)
      (Game|SpawnActorfromClass "/Script/QuartroSemestreSA.Projectile" (Math|Transform|MakeTransform (Math|Vector|MakeVector _x_2 _y_2 225.0) (Math|Rotator|FindLookatRotation _returnvalue_3 (Math|Vector|MakeVector _x _y 225.0)) "0.800000,1.000000,0.800000") "AdjustIfPossibleButAlwaysSpawn" 0 0))))

(event Input|MouseEvents|LeftMouseButton
  (params (Key :type Key%20Structure))
  (bind _returnvalue (Game|GetPlayerController 0))
  (bind _returnvalue_2 (Pawn|GetControlledPawn _returnvalue))
  (bind _hitresult (Game|Player|GetHitResultUnderCursorbyChannel _returnvalue "TraceTypeQuery1" true))
  (bind _returnvalue_3 (Transformation|GetActorLocation _returnvalue_2))
  (bind _location (Collision|BreakHitResult _hitresult))
  (bind (_x _y) (Math|Vector|BreakVector _location))
  (bind (_x_2 _y_2) (Math|Vector|BreakVector _returnvalue_3))
  (:Pressed
    (Utilities|FlowControl|Gate true) ; enters at Open
  )
  (:Released
    (Utilities|FlowControl|Gate true) ; enters at Close
  ))

(fn ConstructionScript)